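; BP_LapManager is a lap-counting actor that detects laps through trigger box overlaps.
; In single player, any overlap increments and prints a lap counter, with no win check.
; Otherwise, BP_Mazda overlaps increment one shared lap count and store that count plus one in a map keyed by controller.
; A win message prints when the shared count equals the total set through ReceiveNumberOfLaps.
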(event `self.TriggerBox.OnComponentBeginOverlap`
  (params (OverlappedComponent :type "PrimitiveComponent Object Reference") (OtherActor :type "Actor Object Reference") (OtherComp :type "PrimitiveComponent Object Reference") (OtherBodyIndex :type Integer) (bFromSweep :type Boolean) (SweepResult :type "HitResult Structure (by ref)"))
  (if (`/Game/BP_GameInstance.IsSinglePlayer` (`/Game/BPFL_Common.GetCarGameGameInstance` self))
    (bind _output_get (set `self.SinglePlayerLapsCounter` (+ (`self.SinglePlayerLapsCounter`) 1)))
    (`KismetSystemLibrary.PrintString` (`KismetStringLibrary.Conv_IntToString` _output_get))
    (else
      (bind _asbp_mazda (cast `/Game/Vehicles/MyCar/Car/BP_Mazda` OtherActor))
      (`self.RegisterPlayerLap` self (`Pawn.GetController` _asbp_mazda)))))

(fn `ReceiveNumberOfLaps`
  (params (NumberOfLaps :type Integer))
  (set `self.TotalNumberOfLaps` NumberOfLaps))

(fn `RegisterPlayerLap`
  (params (ControllerToRegister :type "Controller Object Reference"))
  (set `self.CurrentLapsMade` (+ 1 (`self.CurrentLapsMade`)))
  (`KismetSystemLibrary.PrintText` (`KismetTextLibrary.Conv_ObjectToText` ControllerToRegister))
  (`BlueprintMapLibrary.Map_Add` (`self.PlayerLapTracker`) ControllerToRegister (+ 1 (`self.CurrentLapsMade`)))
  (if (== (`self.CurrentLapsMade`) (`self.TotalNumberOfLaps`))
    (`KismetSystemLibrary.PrintString` "You WOn")))

(fn `UserConstructionScript`)