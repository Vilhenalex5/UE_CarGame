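; BP_CheckPointManager tracks each player's progress through an ordered, looping sequence of checkpoints.
; RegisterPlayer maps a controller to index zero in PlayerCheckpointTracker.
; NotifyCheckpointCrossed compares the crossed checkpoint with that controller's expected entry in Checkpoints, advancing the index on a match and wrapping after the last.
; Wrong checkpoints and unregistered controllers leave progress unchanged, and every outcome only prints a debug string.
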(fn `NotifyCheckpointCrossed`
  (params (Controller :type "Controller Object Reference") (Checkpoint :type "/Game/RacingGame/CheckPoints/BP_Checkpoint Object Reference"))
  (bind (_value _returnvalue) (`BlueprintMapLibrary.Map_Find` (`self.PlayerCheckpointTracker`) Controller))
  (if _returnvalue
    (if (== (`|GetArrayItem` (`self.Checkpoints`) _value) Checkpoint)
      (`BlueprintMapLibrary.Map_Add` (`self.PlayerCheckpointTracker`) (`local.Controller`) (`KismetMathLibrary.Wrap` (+ _value 1) -1 (`KismetArrayLibrary.Array_LastIndex` (`self.Checkpoints`))))
      (`KismetSystemLibrary.PrintString` "GoodBoy")
      (else
        (`KismetSystemLibrary.PrintString` "Bad Boy")))
    (else
      (`KismetSystemLibrary.PrintString` "Failed To Find Player"))))

(fn `RegisterPlayer`
  (params (ControllerToRegister :type "Controller Object Reference"))
  (`BlueprintMapLibrary.Map_Add` (`self.PlayerCheckpointTracker`) ControllerToRegister))

(fn `UserConstructionScript`)