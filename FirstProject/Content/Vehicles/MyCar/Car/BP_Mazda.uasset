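; BP_Mazda is a Chaos wheeled car that adds engine audio, exhaust backfires, a brake light and a lap-win check.
; Tick scales engine sound pitch with RPM and triggers a cooldown-gated pop at high RPM outside reverse, briefly firing two NGFire effects.
; The pop sound uses NGFire1's relative location as its world position.
; The S key toggles the rect light while held, and LapCrossed prints a win on the final lap.
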(event `self.ReceiveBeginPlay`
  (`parent.ReceiveBeginPlay`))

(event `self.ReceiveTick`
  (params (DeltaSeconds :type "Float (single-precision)"))
  (`parent.ReceiveTick` DeltaSeconds)
  (`|ExecutionSequence`
    (:`then_0`
      (`self.CheckRPM`))
    (:`then_1`
      (`AudioComponent.SetPitchMultiplier` (`self.Engine`) (+ (/ (`ChaosWheeledVehicleMovementComponent.GetEngineRotationSpeed` (`self.Chaos Wheeled Vehicle Movement Component`)) 3200.0) 0.1)))))

(event `CheckRPM`
  (if (== (`ChaosVehicleMovementComponent.GetCurrentGear` (`self.VehicleMovementComponent`)) -1)
    _
    (elif (`self.isPopping`)
      _
      (elif (>= (`ChaosWheeledVehicleMovementComponent.GetEngineRotationSpeed` (`self.Chaos Wheeled Vehicle Movement Component`)) 5600.0)
        (set `self.isPopping` true)
        (`self.Pop Effect`)))))

(event `Pop Effect`
  (`GameplayStatics.PlaySoundAtLocation` "/Game/Car_pop.Car_pop" (`SceneComponent.RelativeLocation` (`self.NG_Fire1`)) (struct) 1.0 1.0 0.0 null null null null)
  (`self.Effects`)
  (`KismetSystemLibrary.Delay` 2.0)
  (set `self.isPopping` false))

(event `Effects`
  (`ActorComponent.Activate` (`self.NG_Fire1`) false)
  (`ActorComponent.Activate` (`self.NG_Fire`) false)
  (`KismetSystemLibrary.Delay` 0.2)
  (`ActorComponent.Deactivate` (`self.NG_Fire1`))
  (`ActorComponent.Deactivate` (`self.NG_Fire`)))

(event `Key|S`
  (params (Key :type "Key Structure"))
  (:`Pressed`
    (set `self.IsBreaking` true)
    (`SceneComponent.SetVisibility` (`self.RectLight`) (`self.IsBreaking`) false :!label _label))
  (:`Released`
    (set `self.IsBreaking` false)
    (goto _label)))

(event `LapCrossed`
  (if (== (`self.LapsToFinish`) (`self.CurrentLap`))
    (`KismetSystemLibrary.PrintString` "Player Wins")))

(fn `UserConstructionScript`
  (`parent.UserConstructionScript`))