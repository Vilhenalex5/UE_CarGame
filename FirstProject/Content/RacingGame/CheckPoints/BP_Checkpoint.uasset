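; BP_Checkpoint is a race checkpoint trigger actor that registers when a BP_Mazda car drives through it.
; It finds the level's CheckPointManager on BeginPlay and, on trigger box overlap, notifies it with the car's controller and itself.
; In single-player games, it also tells the countdown timer on that player's vehicle HUD that a checkpoint was crossed.
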(event `self.ReceiveBeginPlay`
  (bind _returnvalue (`GameplayStatics.GetActorOfClass` "/Script/FirstProject.CheckPointManager"))
  (set `self.CheckPointManager` _returnvalue))

(event `self.TriggerBox.OnComponentBeginOverlap`
  (params (OverlappedComponent :type "PrimitiveComponent Object Reference") (OtherActor :type "Actor Object Reference") (OtherComp :type "PrimitiveComponent Object Reference") (OtherBodyIndex :type Integer) (bFromSweep :type Boolean) (SweepResult :type "HitResult Structure (by ref)"))
  (bind _asbp_mazda (cast `/Game/Vehicles/MyCar/Car/BP_Mazda` OtherActor))
  (bind _returnvalue (`Pawn.GetController` _asbp_mazda))
  (`CheckPointManager.NotifyCheckpointCrossed` (`self.CheckPointManager`) _returnvalue self)
  (bind _asvehicle_player_controller (cast `/Game/VehicleTemplate/Blueprints/VehiclePlayerController` _returnvalue))
  (if (`/Game/BP_GameInstance.IsSinglePlayer` (`/Game/BPFL_Common.GetCarGameGameInstance` self))
    (`/Game/CountDownTimer.CheckPointCrossed` (`/Game/VehicleTemplate/Blueprints/VehicleUI.CountDownTimer` (`/Game/VehicleTemplate/Blueprints/VehiclePlayerController.VehicleHud` _asvehicle_player_controller)))))

(fn `UserConstructionScript`)