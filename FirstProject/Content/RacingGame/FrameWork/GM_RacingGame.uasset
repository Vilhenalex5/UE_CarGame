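; Racing game mode that passes the lap count to the race and assigns player spawn points.
; On BeginPlay it sends the game instance's NumberOfLaps to BP_LapManager; the following finish-line checkpoint scan and delay trigger nothing.
; ChoosePlayerStart hands out lazily cached PlayerStarts in array order through an incrementing tracker, with no bounds check, so the level needs enough starts for every player.
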(event `self.ReceiveBeginPlay`
  (`parent.ReceiveBeginPlay`)
  (bind _returnvalue (`GameplayStatics.GetActorOfClass` "/Game/BP_LapManager.BP_LapManager_C"))
  (`/Game/BP_LapManager.ReceiveNumberOfLaps` _returnvalue (`/Game/BP_GameInstance.NumberOfLaps` (`/Game/BPFL_Common.GetCarGameGameInstance` self)))
  (`|ExecutionSequence`
    (:`then_0`
      (bind _outactors (`GameplayStatics.GetAllActorsOfClass` "/Game/RacingGame/CheckPoints/BP_Checkpoint.BP_Checkpoint_C"))
      (for _array_element _outactors
        (if (`/Game/RacingGame/CheckPoints/BP_Checkpoint.IsFinishLine` _array_element)
          _)))
    (:`then_1`
      (`KismetSystemLibrary.Delay` 3.0))))

(fn `ChoosePlayerStart`
  (params (Player :type "Controller Object Reference"))
  (returns (ReturnValue :type "Actor Object Reference"))
  (locals (PlayerStart :type "PlayerStart Object Reference"))
  (bind _spawnpointtracker (`self.SpawnPointTracker`))
  (bind _output_get (set `local.PlayerStart` (`|GetArrayItem` (`self.GetOrFindSpawnPoints`) _spawnpointtracker)))
  (`/Engine/EditorBlueprintResources/StandardMacros.IncrementInt` _spawnpointtracker ; If there is an error here do us both a favour and create enough player starts :p
    (:`  `
      (return _output_get))))

(fn `GetOrFindSpawnPoints`
  (returns (Output_Get :type "Array of PlayerStart Object Reference"))
  (if (`KismetArrayLibrary.Array_IsEmpty` (`self.SpawnPoints`))
    (bind _outactors (`GameplayStatics.GetAllActorsOfClass` "/Script/Engine.PlayerStart"))
    (bind _output_get (set `self.SpawnPoints` _outactors)))
  (return _output_get))

(fn `UserConstructionScript`)